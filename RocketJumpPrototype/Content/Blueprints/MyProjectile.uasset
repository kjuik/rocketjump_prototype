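; MyProjectile is a projectile actor with a sphere and flame that explodes on its first collision.
; The construction script turns on collision, and a DoOnce gate on the Hit event limits the explosion to one trigger.
; On impact it removes the sphere and flame, fires a radial force impulse, spawns explosion particles with attached sound, then destroys itself after a delay.
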(event EventHit
  (params (MyComp :type Primitive%20Component%20Object%20Reference) (Other :type Actor%20Object%20Reference) (OtherComp :type Primitive%20Component%20Object%20Reference) (bSelfMoved :type Boolean) (HitLocation :type Vector :default "0, 0, 0") (HitNormal :type Vector :default "0, 0, 0") (NormalImpulse :type Vector :default "0, 0, 0") (Hit :type Hit%20Result%20Structure%20%28by%20ref%29))
  ;[1 1 1] On first collision
  (Utilities|FlowControl|DoOnce false
    (:Completed
      ;[1 1 1] Hide sphere and particles
      (Components|DestroyComponent (Variables|MyProjectile|GetSphere))
      (Components|DestroyComponent (Variables|Default|GetFlame))
      ;[1 1 1] Spawn force
      (Class|RadialForceComponent|FireImpulse (Variables|Default|GetRadialForce1))
      ;[1 1 1] Spawn Particles
      (bind _returnvalue (Effects|SpawnEmitteratLocation "/Game/Particles/P_Explosion.P_Explosion" (Transformation|GetWorldLocation (Variables|Default|GetRadialForce1))))
      ;[1 1 1] Play Explosion Sound
      (Class|GameplayStatics|PlaySoundAttached "/Game/Audio/Explosion01.Explosion01" _returnvalue)
      ;[1 1 1] Destroy after Delay
      (Utilities|FlowControl|Delay 5.0)
      (Actor|DestroyActor))))

(fn ConstructionScript
  (CallFunction|EnableCollision))

(fn EnableCollision
  (Variables|Default|SetcanCollide true))